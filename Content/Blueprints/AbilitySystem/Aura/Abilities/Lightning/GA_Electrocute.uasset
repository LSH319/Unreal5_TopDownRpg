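; Electrocute gameplay ability: a channeled lightning spell for Aura, aimed at the mouse and held until input release.
; Target data hides the cursor, turns the avatar, fires a burst cue and plays the montage.
; A montage event disables movement and starts the shock-loop cue, attached to the weapon and targeted at socket height.
; Release restores cursor and walking, removes the loop cue and ends the ability; no damage is applied here.
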(event `self.K2_ActivateAbility`
  (bind _returnvalue (`self.GetAvatarActorFromActorInfo`))
  (bind (_mousehitlocation_x _mousehitlocation_y) (`KismetMathLibrary.BreakVector` (`self.MouseHitLocation`)))
  (if (`KismetSystemLibrary.DoesImplementInterface` (`self.GetAvatarActorFromActorInfo`) "/Script/Aura.CombatInterface")
    (bind (_asynctaskproxy _datahandle) (`TargetDataUnderMouse.CreateTargetDataUnderMouse`)
      (:`ValidData`
        (`self.StoreMouseDataInfo` (`AbilitySystemBlueprintLibrary.GetHitResultFromTargetData` _datahandle))
        (`self.StoreOwnerVariables`)
        (`|ExecutionSequence`
          (:`then_0`
            (set `PlayerController.bShowMouseCursor` false (`self.OwnerPlayerController`))
            (message `CombatInterface.UpdateFacingTarget` (`self.GetAvatarActorFromActorInfo`) (`self.MouseHitLocation`))
            (`self.K2_ExecuteGameplayCue` (struct :`TagName` "GameplayCue.ShockBurst"))
            (`AbilityTask_PlayMontageAndWait.CreatePlayMontageAndWaitProxy` "None" (`self.Montage_Electocute`) 1.0 "None" false
              (:`then`
                (`AbilityTask_WaitGameplayEvent.WaitGameplayEvent` (struct :`TagName` "Event.Montage.Electrocute") null
                  (:`EventReceived`
                    (`self.InShockLoop`)
                    (bind _returnvalue_2 (message `CombatInterface.GetWeapon` _returnvalue))
                    (bind (_returnvalue_x _returnvalue_y _returnvalue_z) (`KismetMathLibrary.BreakVector` (`SceneComponent.GetSocketLocation` _returnvalue_2 "TipSocket")))
                    (`GameplayCueFunctionLibrary.AddGameplayCueOnActor` _returnvalue (struct :`TagName` "GameplayCue.ShockLoop") (`AbilitySystemBlueprintLibrary.MakeGameplayCueParameters` 0.0 0.0 (struct) (struct) (struct) (struct) (struct) (`KismetMathLibrary.MakeVector` _mousehitlocation_x _mousehitlocation_y _returnvalue_z) (0.0 0.0 0.0) null null null null 1 1 _returnvalue_2)))))))
          (:`then_1`
            (`AbilityTask_WaitInputRelease.WaitInputRelease` false
              (:`OnRelease`
                (`self.Prepare to End Ability`)
                (`self.K2_RemoveGameplayCue` (struct :`TagName` "GameplayCue.ShockLoop"))
                (`self.K2_EndAbility`)))))))
    (else
      (`self.K2_EndAbility`))))

(fn `InShockLoop`
  (message `CombatInterface.SetInShockLoop` (`self.GetAvatarActorFromActorInfo`) true)
  (`CharacterMovementComponent.DisableMovement` (`Character.CharacterMovement` (`self.OwnerCharacter`))))

(fn `Prepare to End Ability`
  (set `PlayerController.bShowMouseCursor` true (`self.OwnerPlayerController`))
  (message `CombatInterface.SetInShockLoop` (`self.GetAvatarActorFromActorInfo`) false)
  (`CharacterMovementComponent.SetMovementMode` (`Character.CharacterMovement` (`self.OwnerCharacter`)) "MOVE_Walking" 0))